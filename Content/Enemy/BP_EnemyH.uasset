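; BP_EnemyH is an enemy Blueprint that sets a horizontal movement direction along its right vector.
; BeginPlay starts it facing right, and overlapping an actor tagged "Lateral" toggles IsRight.
; MovementDirection is set to the negated right vector only when IsRight turns false; the true case leaves it unchanged.
; No movement is applied here, and Tick is disabled.
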(event EventBeginPlay
  (|CallParentFunction)
  (Variables|Default|SetMovementDirection (Transformation|GetActorRightVector))
  (Variables|Default|SetisRight true))

(event Collision|EventActorBeginOverlap
  (params (OtherActor :type Actor%20Object%20Reference))
  (|CallParentFunction OtherActor)
  (if (Utilities|Array|ContainsItem (Variables|/Script/Engine.Actor|GetTags OtherActor) "Lateral")
    (bind _output_get (Variables|Default|SetisRight (not (Variables|Default|GetisRight))))
    (if (not _output_get)
      (Variables|Default|SetMovementDirection (* (Transformation|GetActorRightVector) -1)))))

(event EventTick
  (params (DeltaSeconds :type Float%20%28single-precision%29))
  (|CallParentFunction DeltaSeconds) ; This node is disabled and will not be called.\nDrag off pins to build functionality.
)

(fn ConstructionScript
  (|CallParentFunction))