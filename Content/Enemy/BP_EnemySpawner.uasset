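; BP_EnemySpawner periodically spawns enemies in the level from object pools.
; On BeginPlay a looping timer, with a short start delay, fires SpawnEnemy at the TimeToSpawn interval.
; Each spawn randomly picks one of three pools (base, double-shoot or sinus enemies) and places the enemy at the transform of a random component tagged EnemySpawnPoint.
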(event Custom|ReadyToSpawn
  (CallFunction|SpawnEnemy))

(event EventBeginPlay
  (Utilities|Time|SetTimerbyEvent (delegate Custom|ReadyToSpawn) (Variables|Default|GetTimeToSpawn) true false 3.0))

(event Collision|EventActorBeginOverlap
  (params (OtherActor :type Actor%20Object%20Reference)))

(event EventTick
  (params (DeltaSeconds :type Float%20%28single-precision%29)))

(fn ConstructionScript)

(fn SpawnEnemy
  (bind _returnvalue (Actor|GetComponentsbyTag "/Script/Engine.SceneComponent" "EnemySpawnPoint"))
  (Default|SpawnfromPool (Utilities|Select :Index (Math|Random|RandomInteger 3) :Option%200 (Variables|Default|GetBaseEnemiesPool) :Option%201 (Variables|Default|GetDoubleShootEnemiesPool) :Option%202 (Variables|Default|GetSinusEnemiesPool)) (Transformation|GetWorldTransform (Utilities|Array|Get(acopy) _returnvalue (Math|Random|RandomInteger (Utilities|Array|Length _returnvalue))))))