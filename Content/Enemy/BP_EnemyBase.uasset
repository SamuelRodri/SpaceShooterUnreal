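; Base enemy for a shooter that flies straight along its starting forward vector and fires on a cooldown.
; Tick moves it without sweep and accumulates a shoot timer, spawning AmmoType at every FirePoint-tagged component with the enemy's rotation.
; Overlapping a Player-tagged actor adds score through MyGameMode, plays explosion effects and calls OnEnemyDestroy.
; That bound event marks the enemy not in use rather than destroying it, suggesting pooling.
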(event Custom|DestroyEvent
  ;[1 1 1] Enemy Setup
  (CallFunction|SetinUse false))

(event EventBeginPlay
  ;[1 1 1] Enemy Setup
  (Variables|Default|SetMovementDirection (Transformation|GetActorForwardVector))
  (EventDispatchers|BindEventtoOnEnemyDestroy (delegate Custom|DestroyEvent)))

(event Collision|EventActorBeginOverlap
  (params (OtherActor :type Actor%20Object%20Reference))
  ;[1 1 1] Enemy Hit
  (if (Utilities|Array|ContainsItem (Variables|/Script/Engine.Actor|GetTags OtherActor) "Player")
    (bind _asmy_game_mode (Utilities|Casting|CastToMyGameMode (Game|GetGameMode)))
    (Default|IncreseScore _asmy_game_mode (Variables|Default|GetScoreWhenDestroy))
    (Effects|SpawnEmitteratLocation "/Game/StarterContent/Particles/P_Explosion.P_Explosion" (Transformation|GetActorLocation))
    (Audio|PlaySound2D "/Game/StarterContent/Audio/Explosion01.Explosion01" 1.0 1.0 0.0 0 0)
    (Default|CallOnEnemyDestroy)))

(event EventTick
  (params (DeltaSeconds :type Float%20%28single-precision%29))
  ;[1 1 1] Enemy Behaviour
  (CallFunction|Move DeltaSeconds)
  (bind _shoottimer (CallFunction|UpdateShootTimer DeltaSeconds))
  (if (>= _shoottimer (Variables|Default|GetFireCoolDown))
    (Variables|Default|SetShootTimer 0.0)
    (CallFunction|Fire)))

(fn ConstructionScript)

(fn Move
  (params (DeltaTime :type Float%20%28double-precision%29))
  (Transformation|SetActorLocation (+ (Transformation|GetActorLocation) (* (* DeltaTime (Variables|Default|GetSpeed)) (Variables|Default|GetMovementDirection))) false false))

(fn Fire
  (bind _arrayelement (Utilities|Array|ReverseforEachLoop (Actor|GetComponentsbyTag "/Script/Engine.SceneComponent" "FirePoint"))
    (:LoopBody
      (bind _returnvalue (Game|SpawnActorfromClass (Variables|Default|GetAmmoType) (Math|Conversions|ToTransform(Vector) (Transformation|GetWorldLocation _arrayelement)) "Undefined" "MultiplyWithRoot" 0 0))
      (Transformation|SetActorRotation _returnvalue (Transformation|GetActorRotation))
      (Audio|PlaySound2D "/Game/Audio/Sci-Fi_Shots_Pack2_Game_Of_Weapons/Wave/SciFi_Shot_P2__141_.SciFi_Shot_P2__141_" 1.0 1.0 0.0 0 0))))

(fn UpdateShootTimer
  (params (Elapsed%20Time :type Float%20%28double-precision%29))
  (bind _output_get (Variables|Default|SetShootTimer (+ Elapsed%20Time (Variables|Default|GetShootTimer))))
  (return _output_get))