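; Pooled enemy Blueprint that weaves along a sine path while firing on a cooldown, building on a parent enemy class.
; Tick moves it along MovementDirection, recomputes the Y component from a sine of its lifetime and right vector, then updates the shoot timer.
; Overlapping a Player-tagged actor fires the destroy dispatcher, which clears its in-use state; an additional Lateral tag on that actor reverses direction.
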(event Custom|DestroyEvent
  ;[1 1 1] Enemy Setup
  (CallFunction|SetinUse false))

(event EventBeginPlay
  ;[1 1 1] Enemy Setup
  (Variables|Default|SetMovementDirection "1.000000,1.000000,0.000000")
  (EventDispatchers|BindEventtoOnEnemyDestroy0 (delegate Custom|DestroyEvent)))

(event Collision|EventActorBeginOverlap
  (params (OtherActor :type Actor%20Object%20Reference))
  (bind _tags (Variables|/Script/Engine.Actor|GetTags OtherActor))
  ;[1 1 1] Enemy Hit
  (|CallParentFunction OtherActor)
  (if (Utilities|Array|ContainsItem _tags "Player")
    (Default|CallOnEnemyDestroy0)
    (if (Utilities|Array|ContainsItem _tags "Lateral")
      (Variables|Default|SetMovementDirection (* (Variables|Default|GetMovementDirection) -1)))))

(event EventTick
  (params (DeltaSeconds :type Float%20%28single-precision%29))
  ;[1 1 1] Enemy Behaviour
  (CallFunction|Move DeltaSeconds)
  (bind _shoottimer (CallFunction|UpdateShootTimer DeltaSeconds))
  (if (>= _shoottimer (Variables|Default|GetFireCoolDown))
    (Variables|Default|SetShootTimer 0.0)
    (CallFunction|Fire)))

(fn ConstructionScript)

(fn Move
  (params (DeltaTime :type Float%20%28double-precision%29))
  (Transformation|SetActorLocation (+ (Transformation|GetActorLocation) (* (* DeltaTime (Variables|Default|GetSpeed)) (Variables|Default|GetMovementDirection))) false false)
  (Variables|Default|SetMovementDirection (Math|Vector|MakeVector (.x (Variables|Default|GetMovementDirection)) (.y (* (Math|Trig|Sin(Degrees) (* (Actor|GetGameTimeSinceCreation) 1.5e+02)) (Transformation|GetActorRightVector))) (.z (Variables|Default|GetMovementDirection)))))