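; BP_SpaceSBaseAmmo is a base projectile actor, apparently for a space shooter, that flies straight and explodes on contact with tagged targets.
; Each tick, Move offsets its location along the forward vector by Speed scaled by delta time, without sweeping.
; When it overlaps an actor carrying TargetTag, it spawns an explosion emitter, plays a 2D sound, then destroys itself after a short delay.
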(event Collision|EventActorBeginOverlap
  (params (OtherActor :type Actor%20Object%20Reference))
  ;[1 1 1] Ammo Hit
  (if (Utilities|Array|ContainsItem (Variables|/Script/Engine.Actor|GetTags OtherActor) (Variables|Default|GetTargetTag))
    (Effects|SpawnEmitteratLocation "/Game/StarterContent/Particles/P_Explosion.P_Explosion" (Transformation|GetActorLocation))
    (Audio|PlaySound2D "/Game/StarterContent/Audio/Explosion01.Explosion01" 1.0 1.0 0.0 0 0)
    (Utilities|FlowControl|Delay 0.2)
    (Actor|DestroyActor)))

(event EventTick
  (params (DeltaSeconds :type Float%20%28single-precision%29))
  ;[1 1 1] Ammo Movement
  (CallFunction|Move DeltaSeconds))

(fn ConstructionScript)

(fn Move
  (params (Delta%20Time :type Float%20%28single-precision%29))
  (Transformation|SetActorLocation (+ (Transformation|GetActorLocation) (* (* Delta%20Time (Variables|Default|GetSpeed)) (Transformation|GetActorForwardVector))) false false))